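; DronePawn is a suicide drone that patrols linked PatrolPoints, chases an FPS_Character and explodes on contact.
; AI MoveTo drives the patrol, following each NextPoint after a short delay, until a Sphere overlap makes the character the new goal.
; Overlapping the Explodes component damages the character, and that or depleted health calls Explode for sound, particles and self-destruction.
; Tick smoothly turns the drone toward its current goal.
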(event `self.ReceiveBeginPlay`
  (bind _goal_actor (`self.Goal Actor`))
  (add `self.OnTakeAnyDamage` (delegate `OnTakeDamage`))
  (`/Engine/EditorBlueprintResources/StandardMacros.IsValid` _goal_actor :!label _label
    (:`Is Valid`
      (`AITask_MoveTo.AIMoveTo` (`AIBlueprintHelperLibrary.GetAIController` self) (0.0 0.0 0.0) _goal_actor 25.0 "Disable"
        (:`OnMoveFinished`
          (bind _aspatrol_point (cast `/Game/Blueprints/Drone/PatrolPoint` (`self.Goal Actor`)))
          (set `self.Goal Actor` (`/Game/Blueprints/Drone/PatrolPoint.NextPoint` _aspatrol_point))
          (`KismetSystemLibrary.Delay` 1.0)
          (goto _label))))))

(event `OnTakeDamage` :!signature `self.OnTakeAnyDamage`
  (params (DamagedActor :type "Actor Object Reference") (Damage :type "Float (single-precision)") (DamageType :type "DamageType Object Reference") (InstigatedBy :type "Controller Object Reference") (DamageCauser :type "Actor Object Reference"))
  (bind _output_get (set `self.Health` (- (`self.Health`) Damage)))
  (if (<= _output_get 0.0)
    (`self.Explode`)))

(event `Move to Goal Target`
  (params (NewParam :type "Actor Object Reference"))
  (bind _output_get (set `self.Goal Actor` NewParam))
  (`|AIMoveTo` self (0.0 0.0 0.0) _output_get 50.0))

(event `self.Sphere.OnComponentBeginOverlap`
  (params (OverlappedComponent :type "PrimitiveComponent Object Reference") (OtherActor :type "Actor Object Reference") (OtherComp :type "PrimitiveComponent Object Reference") (OtherBodyIndex :type Integer) (bFromSweep :type Boolean) (SweepResult :type "HitResult Structure (by ref)"))
  (bind _asfps_character (cast `/Game/Blueprints/Character/FPS_Character` OtherActor))
  (`self.Move to Goal Target` _asfps_character))

(event `self.Explodes.OnComponentBeginOverlap`
  (params (OverlappedComponent :type "PrimitiveComponent Object Reference") (OtherActor :type "Actor Object Reference") (OtherComp :type "PrimitiveComponent Object Reference") (OtherBodyIndex :type Integer) (bFromSweep :type Boolean) (SweepResult :type "HitResult Structure (by ref)"))
  (bind _asfps_character (cast `/Game/Blueprints/Character/FPS_Character` OtherActor))
  (`GameplayStatics.ApplyDamage` _asfps_character (`self.Damage`))
  (`self.Explode`))

(event `self.ReceiveTick`
  (params (DeltaSeconds :type "Float (single-precision)"))
  (bind _goal_actor (`self.Goal Actor`))
  (`/Engine/EditorBlueprintResources/StandardMacros.IsValid` _goal_actor
    (:`Is Valid`
      (`self.K2_SetActorRotation` (`KismetMathLibrary.RInterpTo` (`self.K2_GetActorRotation`) (`KismetMathLibrary.FindLookAtRotation` (`self.K2_GetActorLocation`) (`self.K2_GetActorLocation` _goal_actor)) DeltaSeconds 6.0)))))

(fn `Explode`
  (bind _returnvalue (`self.K2_GetActorLocation`))
  (`GameplayStatics.PlaySoundAtLocation` "/Game/StarterContent/Audio/Explosion_Cue.Explosion_Cue" _returnvalue (struct) 1.0 1.0 0.0 null null null null)
  (`GameplayStatics.SpawnEmitterAtLocation` "/Game/StarterContent/Particles/P_Explosion.P_Explosion" _returnvalue (struct) (3.0 3.0 3.0))
  (`self.K2_DestroyActor`))

(fn `UserConstructionScript`)